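; BP_Turret is a turret actor that aims and fires projectiles at the first player's pawn while it is within TurretDistance.
; Each Tick checks range and snaps the Sphere component to a look-at rotation computed from the Cube's location.
; A Delay of TimeBetweenShots on the same Tick path throttles firing, then spawns a Projectile at the Arrow component's world transform.
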(event `self.ReceiveTick`
  (params (DeltaSeconds :type "Float (single-precision)"))
  ;[1 1 1] Checks the distance to the player
  (if (< (`self.GetDistanceTo` (`GameplayStatics.GetPlayerPawn` 0)) (`self.TurretDistance`))
    ;[1 1 1] Follows the Player
    (`SceneComponent.K2_SetWorldRotation` (`self.Sphere`) (`KismetMathLibrary.FindLookAtRotation` (`SceneComponent.K2_GetComponentLocation` (`self.Cube`)) (`self.K2_GetActorLocation` (`GameplayStatics.GetPlayerPawn` 0))) false false)
    ;[1 1 1] Spawns the Projectile
    (`KismetSystemLibrary.Delay` (`self.TimeBetweenShots`))
    (`|SpawnActorFromClass` "/Game/BP/Objects/Projectile.Projectile_C" (`SceneComponent.K2_GetComponentToWorld` (`self.Arrow`)) "Undefined" "MultiplyWithRoot" null null)))

(fn `UserConstructionScript`)